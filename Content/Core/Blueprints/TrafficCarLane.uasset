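; Traffic lane actor that moves a set of car meshes along a spline.
; BeginPlay adds copies of the master mesh with random CarColor dynamic materials, weighted toward white by repeated palette entries.
; The Traffic timeline spaces cars evenly along the spline, wrapping distances past its end, while Drive is true.
; Tick syncs the timeline's play rate to DrivingSpeed, resetting its time whenever they differ.
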(event `self.ReceiveBeginPlay`
  (bind _carmeshes (`self.CarMeshes`))
  (bind _spline (`self.Spline`))
  (bind _returnvalue (`SceneComponent.GetRelativeTransform` (`self.MasterMesh`)))
  (bind _returnvalue_2 (`SplineComponent.GetSplineLength` _spline))
  (bind _array (`|MakeArray` (`KismetMathLibrary.MakeColor` 0.0) (struct :`R` 1.0 :`G` 1.0 :`B` 1.0 :`A` 1.0) (struct :`R` 0.494792 :`G` 0.494792 :`B` 0.494792 :`A` 1.0) (struct :`R` 1.0 :`G` 0.739732 :`A` 1.0) (struct :`R` 1.0 :`G` 0.007021 :`A` 1.0) (struct :`G` 0.001431 :`B` 0.494792 :`A` 1.0) (struct :`G` 0.078125 :`B` 0.010308 :`A` 1.0) (struct :`R` 0.098958 :`G` 0.044613 :`B` 0.015462 :`A` 1.0) (struct :`R` 1.0 :`G` 1.0 :`B` 1.0 :`A` 1.0) (struct :`R` 1.0 :`G` 1.0 :`B` 1.0 :`A` 1.0) (struct :`R` 1.0 :`G` 1.0 :`B` 1.0 :`A` 1.0) (struct :`R` 1.0 :`G` 1.0 :`B` 1.0 :`A` 1.0) (struct :`R` 1.0 :`G` 1.0 :`B` 1.0 :`A` 1.0) (struct) (struct)))
  (set `self.CarMeshes` (`|MakeArray` (`self.MasterMesh`)))
  (for _ (range 2 (+ (`self.NumberOfCars`) 1))
    (bind _returnvalue_3 (`AddComponent|NODE_AddStaticMeshComponent-0` :`RelativeTransform` _returnvalue))
    (bind _returnvalue_4 (`StaticMeshComponent.SetStaticMesh` _returnvalue_3 "/Game/Core/Meshes/car.car"))
    (if _returnvalue_4
      (bind _returnvalue_5 (`PrimitiveComponent.CreateDynamicMaterialInstance` _returnvalue_3 0 "/Game/Core/Materials/Car.Car" "None"))
      (`MaterialInstanceDynamic.SetVectorParameterValue` _returnvalue_5 "CarColor" (`|GetArrayItem` _array (`KismetMathLibrary.RandomIntegerInRange` 0 (`KismetArrayLibrary.Array_Length` _array))))
      (`KismetArrayLibrary.Array_Add` (`self.CarMeshes`) _returnvalue_3)
      (`PrimitiveComponent.SetBoundsScale` _returnvalue_3 1000.0)))
  (bind (_direction _percentcomplete) (`Timeline|Traffic` :!label _label)
    (:`Update`
      (if (`self.Drive`)
        (for (_array_element _array_index) _carmeshes
          (bind _returnvalue_6 (+ (* _array_index (/ _returnvalue_2 (`KismetArrayLibrary.Array_Length` _carmeshes))) (* _percentcomplete _returnvalue_2)))
          (`SceneComponent.K2_SetWorldTransform` _array_element (`KismetMathLibrary.MakeTransform` (.location (`SplineComponent.GetTransformAtDistanceAlongSpline` _spline (select `bool` (> _returnvalue_6 _returnvalue_2) :`false` _returnvalue_6 :`true` (- _returnvalue_6 _returnvalue_2)) "World" false)) (.rotation (`SplineComponent.GetTransformAtDistanceAlongSpline` _spline (select `bool` (> _returnvalue_6 _returnvalue_2) :`false` _returnvalue_6 :`true` (- _returnvalue_6 _returnvalue_2)) "World" false)) (.scale _returnvalue)) false true))))))

(event `self.ReceiveTick`
  (params (DeltaSeconds :type "Float (single-precision)"))
  (bind _drivingspeed (`self.DrivingSpeed`))
  (bind _traffic (`self.Traffic`))
  (if (!= (`TimelineComponent.GetPlayRate` _traffic) _drivingspeed)
    (`TimelineComponent.SetPlayRate` _traffic _drivingspeed)
    (goto _label :!via `SetNewTime`)))

(fn `UserConstructionScript`)