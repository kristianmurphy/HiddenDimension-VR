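; Player controller that lets the player adjust world-bending parameters in the MPC_WorldManip material parameter collection at runtime.
; BeginPlay caches the collection's values as local targets; held keys step both bend angles (F/R, G/T) and scale the first bend direction (H/Y) per frame.
; Tick spring-interpolates both angles and directions toward those targets and writes them back, using a freshly made spring state each call.
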(event `self.ReceiveBeginPlay`
  (bind _returnvalue (`KismetMaterialLibrary.GetScalarParameterValue` "/Game/Core/MPC_WorldManip.MPC_WorldManip" "BendAngle1"))
  (set `self.BendAngle1Local` _returnvalue)
  (bind _returnvalue_2 (`KismetMaterialLibrary.GetScalarParameterValue` "/Game/Core/MPC_WorldManip.MPC_WorldManip" "BendAngle2"))
  (set `self.BendAble2Local` _returnvalue_2)
  (bind _returnvalue_3 (`KismetMaterialLibrary.GetScalarParameterValue` "/Game/Core/MPC_WorldManip.MPC_WorldManip" "SmoothDistance"))
  (set `self.SmoothDistance` _returnvalue_3)
  (bind _returnvalue_4 (`KismetMaterialLibrary.GetVectorParameterValue` "/Game/Core/MPC_WorldManip.MPC_WorldManip" "BendAxis1"))
  (set `self.BendAxis1Local` (`KismetMathLibrary.Conv_LinearColorToVector` _returnvalue_4))
  (bind _returnvalue_5 (`KismetMaterialLibrary.GetVectorParameterValue` "/Game/Core/MPC_WorldManip.MPC_WorldManip" "BendDirection1"))
  (set `self.BendDirection1Local` (`KismetMathLibrary.Conv_LinearColorToVector` _returnvalue_5))
  (bind _returnvalue_6 (`KismetMaterialLibrary.GetVectorParameterValue` "/Game/Core/MPC_WorldManip.MPC_WorldManip" "BendDirection2"))
  (set `self.BendDirection2Local` (`KismetMathLibrary.Conv_LinearColorToVector` _returnvalue_6)))

(event `self.ReceiveTick`
  (params (DeltaSeconds :type "Float (single-precision)"))
  (set `self.Delta Seconds` DeltaSeconds)
  (`|ExecutionSequence`
    (:`then_0`
      (`|ExecutionSequence`
        (:`then_0`
          (if (`self.IsInputKeyDown` "F")
            (set `self.BendAngle1Local` (+ -2.0 (`self.BendAngle1Local`)))))
        (:`then_1`
          (if (`self.IsInputKeyDown` "R")
            (set `self.BendAngle1Local` (+ 2.0 (`self.BendAngle1Local`)))))
        (:`then_2`
          (if (`self.IsInputKeyDown` "G")
            (set `self.BendAble2Local` (+ -2.0 (`self.BendAble2Local`)))))
        (:`then_3`
          (if (`self.IsInputKeyDown` "T")
            (set `self.BendAble2Local` (+ 2.0 (`self.BendAble2Local`)))))
        (:`then_4`
          (if (`self.IsInputKeyDown` "H")
            (set `self.BendDirection1Local` (* (1.1 1.1 1.1) (`self.BendDirection1Local`)))))
        (:`then_5`
          (if (`self.IsInputKeyDown` "Y")
            (set `self.BendDirection1Local` (* (0.9 0.9 0.9) (`self.BendDirection1Local`)))))))
    (:`then_1`
      (`|ExecutionSequence`
        (:`then_0`
          (bind _returnvalue (`KismetMaterialLibrary.GetScalarParameterValue` "/Game/Core/MPC_WorldManip.MPC_WorldManip" "BendAngle1"))
          (bind _returnvalue_2 (`KismetMathLibrary.FloatSpringInterp` _returnvalue (`self.BendAngle1Local`) (make `FloatSpringState`) 10.0 0.8 (`self.Delta Seconds`)))
          (`KismetMaterialLibrary.SetScalarParameterValue` "/Game/Core/MPC_WorldManip.MPC_WorldManip" "BendAngle1" _returnvalue_2))
        (:`then_1`
          (bind _returnvalue_3 (`KismetMaterialLibrary.GetScalarParameterValue` "/Game/Core/MPC_WorldManip.MPC_WorldManip" "BendAngle2"))
          (bind _returnvalue_4 (`KismetMathLibrary.FloatSpringInterp` _returnvalue_3 (`self.BendAble2Local`) (make `FloatSpringState`) 10.0 0.8 (`self.Delta Seconds`)))
          (`KismetMaterialLibrary.SetScalarParameterValue` "/Game/Core/MPC_WorldManip.MPC_WorldManip" "BendAngle2" _returnvalue_4))
        (:`then_2`
          (bind _returnvalue_5 (`KismetMaterialLibrary.GetVectorParameterValue` "/Game/Core/MPC_WorldManip.MPC_WorldManip" "BendDirection1"))
          (bind _returnvalue_6 (`KismetMathLibrary.VectorSpringInterp` (`KismetMathLibrary.Conv_LinearColorToVector` _returnvalue_5) (`self.BendDirection1Local`) (make `VectorSpringState`) 15.0 0.75 (`self.Delta Seconds`) 0.6))
          (`KismetMaterialLibrary.SetVectorParameterValue` "/Game/Core/MPC_WorldManip.MPC_WorldManip" "BendDirection1" (`KismetMathLibrary.Conv_VectorToLinearColor` _returnvalue_6)))
        (:`then_3`
          (bind _returnvalue_7 (`KismetMaterialLibrary.GetVectorParameterValue` "/Game/Core/MPC_WorldManip.MPC_WorldManip" "BendDirection2"))
          (bind _returnvalue_8 (`KismetMathLibrary.VectorSpringInterp` (`KismetMathLibrary.Conv_LinearColorToVector` _returnvalue_7) (`self.BendDirection2Local`) (make `VectorSpringState`) 15.0 0.75 (`self.Delta Seconds`) 0.6))
          (`KismetMaterialLibrary.SetVectorParameterValue` "/Game/Core/MPC_WorldManip.MPC_WorldManip" "BendDirection2" (`KismetMathLibrary.Conv_VectorToLinearColor` _returnvalue_8)))))))

(fn `UserConstructionScript`)